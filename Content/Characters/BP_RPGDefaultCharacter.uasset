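; BP_RPGDefaultCharacter is an RPG character that routes Enhanced Input to gameplay abilities, interaction and the inventory HUD.
; Move, jump and kick activate GAS abilities, with walking gated on the IsMoving tag.
; Entering Falling activates the airborne ability, while InteractorComponent handles interaction.
; FootCollider starts with collision disabled, and its overlap handler only filters out self, with no further effect.
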(event `self.ReceiveBeginPlay`
  (`PrimitiveComponent.SetCollisionEnabled` (`self.Foot Collider`) "NoCollision"))

(event `self.K2_OnMovementModeChanged`
  (params (PrevMovementMode :type "EMovementMode Enum" :default "MOVE_None") (NewMovementMode :type "EMovementMode Enum" :default "MOVE_None") (PrevCustomMode :type Byte) (NewCustomMode :type Byte))
  (if (`|EnumEquality` NewMovementMode "MOVE_Falling")
    (`AbilitySystemComponent.TryActivateAbilityByClass` (`self.AbilitySystemComponent`) "/Game/Characters/Ability/GA_Airbone.GA_Airbone_C" true)))

(event `EnhancedInput|/Game/Input/IA_Move`
  (params (ActionValue :type "Vector2D Structure") (ElapsedSeconds :type "Float (double-precision)") (TriggeredSeconds :type "Float (double-precision)") (InputAction :type "InputAction Object Reference" :default "/Game/Input/IA_Move.IA_Move"))
  (bind _abilitysystemcomponent (`self.AbilitySystemComponent`))
  (:`Triggered`
    (`AbilitySystemComponent.TryActivateAbilityByClass` _abilitysystemcomponent "/Game/Characters/Ability/GA_Move.GA_Move_C" true)
    (if (`GameplayTagAssetInterface.HasMatchingGameplayTag` _abilitysystemcomponent (struct :`TagName` "Gameplay.State.IsMoving"))
      (`self.K2_Walk` ActionValue)
      (else
        (`FongcrushBlueprintLibrary.K2_CancelAbility` null "/Game/Characters/Ability/GA_Move.GA_Move_C"))))
  (:`Completed`
    (`FongcrushBlueprintLibrary.K2_CancelAbility` _abilitysystemcomponent "/Game/Characters/Ability/GA_Move.GA_Move_C")))

(event `EnhancedInput|/Game/Input/IA_Interact`
  (params (ActionValue :type Boolean) (ElapsedSeconds :type "Float (double-precision)") (TriggeredSeconds :type "Float (double-precision)") (InputAction :type "InputAction Object Reference" :default "/Game/Input/IA_Interact.IA_Interact"))
  (bind _interactorcomponent (`self.InteractorComponent`))
  (:`Triggered`
    (`InteractorComponent.BeginInteract` _interactorcomponent))
  (:`Completed`
    (`InteractorComponent.EndInteract` _interactorcomponent)))

(event `EnhancedInput|/Game/Input/IA_Jump`
  (params (ActionValue :type Boolean) (ElapsedSeconds :type "Float (double-precision)") (TriggeredSeconds :type "Float (double-precision)") (InputAction :type "InputAction Object Reference" :default "/Game/Input/IA_Jump.IA_Jump"))
  (:`Triggered`
    (`AbilitySystemComponent.TryActivateAbilityByClass` (`self.AbilitySystemComponent`) "/Game/Characters/Ability/GA_Jump.GA_Jump_C" true))
  (:`Completed`
    (`self.StopJumping`)))

(event `EnhancedInput|/Game/Input/IA_Inventory`
  (params (ActionValue :type Boolean) (ElapsedSeconds :type "Float (double-precision)") (TriggeredSeconds :type "Float (double-precision)") (InputAction :type "InputAction Object Reference" :default "/Game/Input/IA_Inventory.IA_Inventory"))
  (:`Triggered`
    (`RPGHUD.ToggleInventory` (`self.HUD`))))

(event `EnhancedInput|/Game/Input/IA_Kick`
  (params (ActionValue :type Boolean) (ElapsedSeconds :type "Float (double-precision)") (TriggeredSeconds :type "Float (double-precision)") (InputAction :type "InputAction Object Reference" :default "/Game/Input/IA_Kick.IA_Kick"))
  (:`Triggered`
    (`AbilitySystemComponent.TryActivateAbilityByClass` (`self.AbilitySystemComponent`) "/Game/Characters/Ability/GA_RFKick.GA_RFKick_C" true)))

(event `self.Foot Collider.OnComponentBeginOverlap`
  (params (OverlappedComponent :type "PrimitiveComponent Object Reference") (OtherActor :type "Actor Object Reference") (OtherComp :type "PrimitiveComponent Object Reference") (OtherBodyIndex :type Integer) (bFromSweep :type Boolean) (SweepResult :type "HitResult Structure (by ref)"))
  (if (!= OtherActor self)
    _))

(fn `UserConstructionScript`)