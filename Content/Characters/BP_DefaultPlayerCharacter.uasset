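; BP_DefaultPlayerCharacter is the player character that turns Enhanced Input actions into Gameplay Ability System activations and UI or interaction calls.
; Move, jump and kick activate their abilities; releasing move cancels walk, and releasing jump stops jumping.
; Entering Falling movement mode triggers the airborne ability.
; Inventory toggles through the HUD, interaction begins and ends on an interactor component, and a getter exposes the move input value.
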(event `self.K2_OnMovementModeChanged`
  (params (PrevMovementMode :type "EMovementMode Enum" :default "MOVE_None") (NewMovementMode :type "EMovementMode Enum" :default "MOVE_None") (PrevCustomMode :type Byte) (NewCustomMode :type Byte))
  (if (`|EnumEquality` NewMovementMode "MOVE_Falling")
    (`AbilitySystemComponent.TryActivateAbilityByClass` (`self.AbilitySystemComponent`) "/Game/Characters/Gameplay/GA_Airbone.GA_Airbone_C" true)))

(event `EnhancedInput|/Game/Inputs/IA_Inventory`
  (params (ActionValue :type Boolean) (ElapsedSeconds :type "Float (double-precision)") (TriggeredSeconds :type "Float (double-precision)") (InputAction :type "InputAction Object Reference" :default "/Game/Inputs/IA_Inventory.IA_Inventory"))
  (:`Triggered`
    (`RPGHUD.ToggleInventory` (`self.HUD`))))

(event `EnhancedInput|/Game/Inputs/IA_Interact`
  (params (ActionValue :type Boolean) (ElapsedSeconds :type "Float (double-precision)") (TriggeredSeconds :type "Float (double-precision)") (InputAction :type "InputAction Object Reference" :default "/Game/Inputs/IA_Interact.IA_Interact"))
  (bind _interactorcomponent (`self.InteractorComponent`))
  (:`Triggered`
    (`InteractorComponent.BeginInteract` _interactorcomponent))
  (:`Completed`
    (`InteractorComponent.EndInteract` _interactorcomponent)))

(event `EnhancedInput|/Game/Inputs/IA_Move`
  (params (ActionValue :type "Vector2D Structure") (ElapsedSeconds :type "Float (double-precision)") (TriggeredSeconds :type "Float (double-precision)") (InputAction :type "InputAction Object Reference" :default "/Game/Inputs/IA_Move.IA_Move"))
  (bind _abilitysystemcomponent (`self.AbilitySystemComponent`))
  (:`Triggered`
    (`AbilitySystemComponent.TryActivateAbilityByClass` _abilitysystemcomponent "/Game/Characters/Gameplay/GA_Walk.GA_Walk_C" true))
  (:`Completed`
    (`FongcrushBlueprintLibrary.K2_CancelAbility` _abilitysystemcomponent "/Game/Characters/Gameplay/GA_Walk.GA_Walk_C")))

(event `EnhancedInput|/Game/Inputs/IA_Jump`
  (params (ActionValue :type Boolean) (ElapsedSeconds :type "Float (double-precision)") (TriggeredSeconds :type "Float (double-precision)") (InputAction :type "InputAction Object Reference" :default "/Game/Inputs/IA_Jump.IA_Jump"))
  (:`Triggered`
    (`AbilitySystemComponent.TryActivateAbilityByClass` (`self.AbilitySystemComponent`) "/Game/Characters/Gameplay/GA_Jump.GA_Jump_C" true))
  (:`Completed`
    (`self.StopJumping`)))

(event `EnhancedInput|/Game/Inputs/IA_Kick`
  (params (ActionValue :type Boolean) (ElapsedSeconds :type "Float (double-precision)") (TriggeredSeconds :type "Float (double-precision)") (InputAction :type "InputAction Object Reference" :default "/Game/Inputs/IA_Kick.IA_Kick"))
  (:`Triggered`
    (`AbilitySystemComponent.TryActivateAbilityByClass` (`self.AbilitySystemComponent`) "/Game/Characters/Gameplay/RFKick/GA_RFKick.GA_RFKick_C" true)))

(fn `GetIAMoveValue`
  (returns (ReturnValue :type "Vector2D Structure"))
  (return (`|GetInputActionValue`)))

(fn `UserConstructionScript`)